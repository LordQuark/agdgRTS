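; RTS commander camera with axis movement, middle-mouse rotation, wheel zoom, and ghost-based building placement.
; BuildThisBuilding spawns a ghost that follows cursor traces through a gated Delay loop, rotates with the wheel, and becomes the real building on a valid left click.
; A looping downward trace every 0.1 seconds snaps the rig to terrain height, ignoring Characters.
; It also creates the commander HUD and toggles the main menu on Tab.
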(event Custom|CheckingTerrainHeight
  (bind _returnvalue (Transformation|GetActorLocation))
  (bind _camera (Variables|Default|GetCamera))
  (bind _returnvalue_2 (Transformation|GetWorldLocation _camera))
  (bind (_x _y) (Math|Vector|BreakVector _returnvalue))
  ;[1 1 1] HeightMapper
  (bind _outhit (Collision|LineTraceByChannel _returnvalue_2 (+ _returnvalue_2 "0, 0,-10000.000000") "TraceTypeQuery1" false 0 "None" :!label _label))
  (Utilities|Casting|CastToCharacter (.HitActor (Collision|BreakHitResult _outhit))
    (:then
      _)
    (:CastFailed
      (Transformation|SetActorLocation (Math|Vector|MakeVector _x _y (.Z (Math|Vector|BreakVector (.Location (Collision|BreakHitResult _outhit))))) false)))
  (Utilities|FlowControl|Delay 0.1)
  (goto _label))

(event EventBuildThisBuilding
  (params (GhostBuilding :type Actor%20Class%20Reference) (ActualBuilding :type Actor%20Class%20Reference))
  (bind _returnvalue (Game|GetPlayerController 0))
  (bind _hitresult (Game|Player|GetHitResultUnderCursorbyChannel _returnvalue "TraceTypeQuery1" true))
  (bind _location (Collision|BreakHitResult _hitresult))
  ;[1 1 1] Building Construction
  (Actor|DestroyActor (Variables|Default|GetGhost%20Building))
  (Variables|Default|SetPlacing%20Building true)
  (bind _returnvalue_2 (Game|SpawnActorfromClass GhostBuilding (Math|Conversions|ToTransform(Vector) _location) false 0 0))
  (Variables|Default|SetGhost%20Building _returnvalue_2)
  (Class|RTSInterface|AmYourCommander(Message) (Variables|Default|GetGhost%20Building) self)
  (Utilities|FlowControl|Sequence
    (:then_0
      (goto _label_2 Open))
    (:then_1
      (Transformation|SetActorLocation (Variables|Default|GetGhost%20Building) _location false :!label _label)
      (Utilities|FlowControl|Delay (Variables|Default|GetTickerDelay))
      (Utilities|FlowControl|Gate true :!label _label_2
        (:Exit
          ;;[1 1 1] Spawn Actual, Destroy Ghost
          (Utilities|FlowControl|Sequence
            (:then_0
              (goto _label))
            (:then_1
              (Utilities|FlowControl|Gate true) ; enters at Open
            )))))))

(event Collision|EventActorBeginOverlap
  (params (OtherActor :type Actor%20Object%20Reference)))

(event EventTick
  (params (DeltaSeconds :type Float%20%28single-precision%29)))

(event EventBeginPlay
  (bind _returnvalue (Game|GetPlayerController 0))
  ;[1 1 1] Begin Play
  (Variables|/Script/Engine.PlayerController|SetbShowMouseCursor _returnvalue true)
  (Variables|/Script/Engine.PlayerController|SetbEnableMouseOverEvents _returnvalue true)
  (CallFunction|CheckingTerrainHeight)
  (if (Variables|Default|GetStartWithUI)
    (CallFunction|SpawnUI)))

(event Input|AxisEvents|InputAxisMoveForward
  (params (AxisValue :type Float%20%28single-precision%29))
  ;[1 1 1] Movement
  (Transformation|AddActorLocalOffset (Math|Vector|MakeVector (* AxisValue (Variables|Default|GetMove%20Speed)) 0.0 0.0) false))

(event Input|AxisEvents|InputAxisMoveRight
  (params (AxisValue :type Float%20%28single-precision%29))
  ;[1 1 1] Movement
  (Transformation|AddActorLocalOffset (Math|Vector|MakeVector 0.0 (* AxisValue (Variables|Default|GetMove%20Speed)) 0.0) false))

(event Input|MouseEvents|MouseX
  (params (AxisValue :type Float%20%28single-precision%29))
  ;[1 1 1] Middle Mouse camera Control
  (Utilities|FlowControl|Gate true
    (:Exit
      (Transformation|AddActorLocalRotation (Class|KismetMathLibrary|MakeRot 0.0 (* AxisValue (Variables|Default|GetRotate%20Speed)) 0.0) false))))

(event Input|MouseEvents|MouseY
  (params (AxisValue :type Float%20%28single-precision%29))
  ;[1 1 1] Middle Mouse camera Control
  (Utilities|FlowControl|Gate true
    (:Exit
      (Transformation|AddLocalRotation (Variables|Default|GetCamera) (Class|KismetMathLibrary|MakeRot (* AxisValue (Variables|Default|GetRotate%20Speed)) 0.0 0.0) false))))

(event Input|MouseEvents|LeftMouseButton
  ;[1 1 1] Building Construction
  ;;[1 1 1] Spawn Actual, Destroy Ghost
  (:Pressed
    (Utilities|FlowControl|Gate true :!label _label
      (:Exit
        ;;;[1 1 1] Terrain Check
        (if (not (Variables|Default|GetBadPlacement))
          (Game|SpawnActorfromClass (stale EventBuildThisBuilding ActualBuilding) (Transformation|GetActorTransform (Variables|Default|GetGhost%20Building)) false 0 0)
          (Actor|DestroyActor (Variables|Default|GetGhost%20Building))
          (Variables|Default|SetPlacing%20Building false)
          (Variables|/Script/Engine.PlayerController|SetbShowMouseCursor (Game|GetPlayerController 0) true)
          (Utilities|FlowControl|Sequence
            (:then_0
              (goto _label Close))
            (:then_1
              (Utilities|FlowControl|Gate true) ; enters at Close
            )))))))

(event Input|KeyboardEvents|Tab
  (:Released
    (CallFunction|MainMenu)))

(event Input|MouseEvents|RightMouseButton
  ;[1 1 1] Building Construction
  ;;[1 1 1] Right Click Cancel
  (:Pressed
    (if (Variables|Default|GetPlacing%20Building)
      (Utilities|FlowControl|Sequence
        (:then_0
          (Utilities|FlowControl|Gate true) ; enters at Close
        )
        (:then_1
          ;;[1 1 1] Spawn Actual, Destroy Ghost
          (Utilities|FlowControl|Gate true) ; enters at Close
        )
        (:then_2
          (Actor|DestroyActor (Variables|Default|GetGhost%20Building))
          (Variables|Default|SetPlacing%20Building false))
        (:then_3
          (Variables|/Script/Engine.PlayerController|SetbShowMouseCursor (Game|GetPlayerController 0) true))))))

(event Input|MouseEvents|MouseWheelUp
  (bind _springarm (Variables|Default|GetSpringArm))
  ;[1 1 1] Mousewheel Zooming
  (:Pressed
    (if (not (Variables|Default|GetPlacing%20Building))
      (if (> (Variables|/Script/Engine.SpringArmComponent|GetTargetArmLength _springarm) 1e+02)
        (Variables|/Script/Engine.SpringArmComponent|SetTargetArmLength _springarm (- (Variables|/Script/Engine.SpringArmComponent|GetTargetArmLength _springarm) (Variables|Default|GetZoom%20Speed)))))))

(event Input|MouseEvents|MouseWheelDown
  (bind _springarm (Variables|Default|GetSpringArm))
  ;[1 1 1] Mousewheel Zooming
  (:Pressed
    (if (not (Variables|Default|GetPlacing%20Building))
      (if (< (Variables|/Script/Engine.SpringArmComponent|GetTargetArmLength _springarm) 3.5e+03)
        (Variables|/Script/Engine.SpringArmComponent|SetTargetArmLength _springarm (+ (Variables|/Script/Engine.SpringArmComponent|GetTargetArmLength _springarm) (Variables|Default|GetZoom%20Speed)))))))

(event Input|KeyboardEvents|C
  (bind _returnvalue (Game|GetPlayerController 0))
  ;[1 1 1] Disable Mouse if Active
  (:Pressed
    (if (Variables|/Script/Engine.PlayerController|GetbShowMouseCursor (Game|GetPlayerController 0))
      ;[1 1 1] Enable/Disable Cursor
      (Variables|/Script/Engine.PlayerController|SetbShowMouseCursor _returnvalue false)
      (else
        (Variables|/Script/Engine.PlayerController|SetbShowMouseCursor _returnvalue true)))))

(event Input|MouseEvents|MiddleMouseButton
  ;[1 1 1] Middle Mouse camera Control
  (:Pressed
    (Utilities|FlowControl|Sequence
      (:then_0
        (Utilities|FlowControl|Gate true) ; enters at Open
      )
      (:then_1
        (Utilities|FlowControl|Gate true) ; enters at Open
      )
      (:then_3
        ;[1 1 1] Building Construction
        ;;[1 1 1] Right Click Cancel
        (if (Variables|Default|GetPlacing%20Building)
          (Utilities|FlowControl|Sequence
            (:then_0
              (Utilities|FlowControl|Gate true) ; enters at Close
            )
            (:then_1
              ;;[1 1 1] Spawn Actual, Destroy Ghost
              (Utilities|FlowControl|Gate true) ; enters at Close
            )
            (:then_2
              (Actor|DestroyActor (Variables|Default|GetGhost%20Building))
              (Variables|Default|SetPlacing%20Building false))
            (:then_3
              (Variables|/Script/Engine.PlayerController|SetbShowMouseCursor (Game|GetPlayerController 0) true)))))
      (:then_4
        (Variables|/Script/Engine.PlayerController|SetbShowMouseCursor (Game|GetPlayerController 0) false))))
  (:Released
    (Utilities|FlowControl|Sequence
      (:then_0
        (Utilities|FlowControl|Gate true) ; enters at Close
      )
      (:then_1
        (Utilities|FlowControl|Gate true) ; enters at Close
      )
      (:then_2
        (Variables|/Script/Engine.PlayerController|SetbShowMouseCursor (Game|GetPlayerController 0) true)))))

(event Input|MouseEvents|MouseWheelUp
  (bind _ghost_building (Variables|Default|GetGhost%20Building))
  ;[1 1 1] Building Construction
  ;;[1 1 1] Rotate Ghost Building
  (:Pressed
    (if (Variables|Default|GetPlacing%20Building)
      (Transformation|SetActorRelativeRotation _ghost_building (Class|KismetMathLibrary|MakeRot 0.0 (+ (.Yaw (Class|KismetMathLibrary|BreakRot (Transformation|GetActorRotation _ghost_building))) 1e+01) 0.0)))))

(event Input|MouseEvents|MouseWheelDown
  (bind _ghost_building (Variables|Default|GetGhost%20Building))
  ;[1 1 1] Building Construction
  ;;[1 1 1] Rotate Ghost Building
  (:Pressed
    (if (Variables|Default|GetPlacing%20Building)
      (Transformation|SetActorRelativeRotation _ghost_building (Class|KismetMathLibrary|MakeRot 0.0 (+ (.Yaw (Class|KismetMathLibrary|BreakRot (Transformation|GetActorRotation _ghost_building))) -1e+01) 0.0)))))

(fn ConstructionScript)

(fn UpdateEcoUI
  (Default|EconomyFunc (Variables|Default|GetCommanderHudvar)))

(fn SpawnUI
  ;[1 1 1] Draw Hud
  (bind _returnvalue (UserInterface|CreateWidget "/Game/HUD/CommanderHUD.CommanderHUD_C" 0 self))
  (Utilities|FlowControl|FlipFlop
    (:A
      (UserInterface|Viewport|AddtoViewport (Variables|Default|GetCommanderHudvar) 0)
      (Variables|Default|SetCommanderHudvar _returnvalue))
    (:B
      (Widget|RemovefromParent (Variables|Default|GetCommanderHudvar)))))

(fn MainMenu
  (if (Variables|Default|GetFirstTimeMenu)
    (Variables|Default|SetFirstTimeMenu false)
    (bind _returnvalue (UserInterface|CreateWidget "/Game/HUD/MainMenu.MainMenu_C" (Game|GetPlayerController 0)))
    (bind _output_get (Variables|Default|SetMainMenuVar _returnvalue))
    (UserInterface|Viewport|AddtoViewport _output_get 0)
    (Variables|Default|SetMainMenuDisplayed true)
    (Widget|SetVisibility (Variables|Default|GetCommanderHudvar) "Hidden")
    (elif (Variables|Default|GetMainMenuDisplayed)
      (Widget|RemovefromParent (Variables|Default|GetMainMenuVar))
      (Variables|Default|SetMainMenuDisplayed false)
      (else
        (UserInterface|Viewport|AddtoViewport (Variables|Default|GetMainMenuVar) 0)
        (Variables|Default|SetMainMenuDisplayed true)))))